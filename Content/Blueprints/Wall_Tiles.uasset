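; Wall tile Blueprint that swaps its mesh material to reflect the AI alert state.
; AIStateChange passes the state to Alert after a short retriggerable delay for Idle, or immediately otherwise.
; Alert applies the caught masked material for Combat and the normal one for Idle or Search for Player.
; Becoming view target requires a ZombieMode game mode and, through a constant-false branch, always applies the caught material.
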(event Custom|AIStateChange
  (params (State :type AI_States%20Enum))
  (switch Utilities|FlowControl|Switch|SwitchonAI_States State
    (:NewEnumerator0
      (Utilities|FlowControl|RetriggerableDelay 0.2))
    (:NewEnumerator1
      _)
    (:NewEnumerator2
      _))
  (CallFunction|Alert State))

(event EventOnBecomeViewTarget
  (params (PC :type Player%20Controller%20Object%20Reference))
  (Utilities|Casting|CastToZombieMode (Game|GetGameMode))
  (if false
    (Rendering|Material|SetMaterial (Variables|Debug|GetStaticMeshComponent) 0 "/Game/Materials/Tile_01_Masked.Tile_01_Masked")
    (else
      (Rendering|Material|SetMaterial (Variables|Debug|GetStaticMeshComponent) 0 "/Game/Materials/Tile_01_Masked_Caught.Tile_01_Masked_Caught"))))

(fn ConstructionScript)

(fn Alert
  (params (State :type AI_States%20Enum))
  (Utilities|FlowControl|Sequence
    (:then_0
      (switch Utilities|FlowControl|Switch|SwitchonAI_States State
        (:NewEnumerator0
          (Variables|Default|SetDMI "/Game/Materials/Tile_01_Masked.Tile_01_Masked" :!label _label))
        (:NewEnumerator1
          (Variables|Default|SetDMI "/Game/Materials/Tile_01_Masked_Caught.Tile_01_Masked_Caught"))
        (:NewEnumerator2
          (goto _label))))
    (:then_1
      (Rendering|Material|SetMaterial (Variables|Debug|GetStaticMeshComponent) 0 (Variables|Default|GetDMI))
      (return))))