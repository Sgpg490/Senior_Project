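; BP_CameraSwitcher is a trigger-pair actor that moves a shared camera when the From and To volumes are crossed.
; The first overlap sets Direction; reaching the other volume saves the camera position and moves it to that direction's offset from the switcher.
; Re-entering the starting volume restores the saved position.
; The camera tracks its owning switcher, releasing the previous one without movement; Camera defaults to the first BP_InitialCamera found.
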(event OnComponentBeginOverlap(From)
  (params (OtherActor :type Actor%20Object%20Reference) (OtherComp :type Primitive%20Component%20Object%20Reference) (OtherBodyIndex :type Integer) (bFromSweep :type Boolean) (SweepResult :type Hit%20Result%20Structure%20%28by%20ref%29))
  (Utilities|DirectionSwitch
    (:None
      (Variables|Default|SetDirection "NewEnumerator1"))
    (:Forward
      (CallFunction|ReleaseCamera false))
    (:Backward
      (CallFunction|CaptureCamera))))

(event OnComponentBeginOverlap(To)
  (params (OtherActor :type Actor%20Object%20Reference) (OtherComp :type Primitive%20Component%20Object%20Reference) (OtherBodyIndex :type Integer) (bFromSweep :type Boolean) (SweepResult :type Hit%20Result%20Structure%20%28by%20ref%29))
  (Utilities|DirectionSwitch
    (:None
      (Variables|Default|SetDirection "NewEnumerator2"))
    (:Forward
      (CallFunction|CaptureCamera))
    (:Backward
      (CallFunction|ReleaseCamera false))))

(fn ConstructionScript
  (Utilities|IsValid (Variables|Default|GetCamera)
    (:Is%20Not%20Valid
      (bind _outactors (Actor|GetAllActorsOfClass "/Game/Blueprints/BP_InitialCamera.BP_InitialCamera_C"))
      (Variables|Default|SetCamera (Utilities|Array|Get(acopy) _outactors)))))

(fn CaptureCamera
  (if (Variables|Default|GetMoved)
    (return)
    (else
      (Variables|Default|SetMoved true)
      ;[1 1 1] Save old camera position set as current switcher.
      (Utilities|SaveOldPosition)
      (Utilities|ReleaseCurrentSwitcher)
      (Utilities|SetCurrentSwitcher)
      ;[1 1 1] Move camera in the appropriate direction
      (Utilities|DirectionSwitch
        (:None
          _)
        (:Forward
          (Utilities|MoveForward))
        (:Backward
          (Utilities|MoveBackward)))
      (return))))

(fn ReleaseCamera
  (params (DoNotMove :type Boolean))
  (LocalVariables|SetL_DoNotMove DoNotMove)
  (if (Variables|Default|GetMoved)
    (Variables|Default|SetMoved false)
    (Variables|Default|SetDirection "NewEnumerator0")
    (if (LocalVariables|GetL_DoNotMove)
      _
      (else
        (Default|MoveCamera (Variables|Default|GetCamera) (Variables|Default|GetPreviousCamPosition))))
    (return)
    (else
      (return))))