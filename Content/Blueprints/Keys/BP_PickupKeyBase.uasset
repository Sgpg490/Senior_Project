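; Base Blueprint for a key pickup, with setup in the Construction Script and no active event logic.
; It creates a dynamic material instance on the first material slot of its static mesh.
; The SpotLight's red, green and blue values drive the matching Gloss and Metal intensity parameters, tying the key's material to its light color.
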(event EventBeginPlay)

(event EventActorBeginOverlap
  (params (OtherActor :type Actor%20Object%20Reference)))

(event EventTick
  (params (DeltaSeconds :type Float%20%28single-precision%29)))

(fn ConstructionScript
  (Variables|Default|SetLightColor (Rendering|Components|Light|GetLightColor (Variables|Default|GetSpotLight)))
  (bind _returnvalue (Rendering|Material|CreateDynamicMaterialInstance (Variables|Default|GetStaticMesh) 0 0 :!class /Script/Engine.PrimitiveComponent))
  (bind _output_get (LocalVariables|SetDMI _returnvalue))
  (Rendering|Material|SetScalarParameterValue _output_get "R Gloss Int" (.r (Variables|Default|GetLightColor)) :!class /Script/Engine.MaterialInstanceDynamic)
  (Rendering|Material|SetScalarParameterValue (LocalVariables|GetDMI) "R Metal Int" (.r (Variables|Default|GetLightColor)) :!class /Script/Engine.MaterialInstanceDynamic)
  (Rendering|Material|SetScalarParameterValue _output_get "G Gloss Int" (.g (Variables|Default|GetLightColor)) :!class /Script/Engine.MaterialInstanceDynamic)
  (Rendering|Material|SetScalarParameterValue (LocalVariables|GetDMI) "G Metal Int" (.g (Variables|Default|GetLightColor)) :!class /Script/Engine.MaterialInstanceDynamic)
  (Rendering|Material|SetScalarParameterValue _output_get "B Gloss Int" (.b (Variables|Default|GetLightColor)) :!class /Script/Engine.MaterialInstanceDynamic)
  (Rendering|Material|SetScalarParameterValue (LocalVariables|GetDMI) "B Metal Int" (.b (Variables|Default|GetLightColor)) :!class /Script/Engine.MaterialInstanceDynamic))