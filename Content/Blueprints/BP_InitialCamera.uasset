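; BP_InitialCamera is a camera actor that registers itself as the static camera on BeginPlay and can glide to new positions.
; Tick passes delta time to UpdateStaticCamera, whose logic lives outside this graph.
; MoveCamera stores the camera component's world location as the start, then plays the Movement timeline from the beginning to lerp the actor's location to the requested destination, without sweep.
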(event Custom|MoveCamera
  (params (NewLocation :type Vector))
  (Variables|Default|SetDestination NewLocation)
  (Variables|Default|SetSource (Transformation|GetWorldLocation (Variables|CameraActor|GetCameraComponent)))
  (bind _location (Timeline|Movement PlayFromStart)
    (:Update
      (Transformation|SetActorLocation (Math|Vector|Lerp(Vector) (Variables|Default|GetSource) (Variables|Default|GetDestination) _location) false false))))

(event EventBeginPlay
  (CallFunction|SetStaticCamera self))

(event EventActorBeginOverlap
  (params (OtherActor :type Actor%20Object%20Reference)))

(event EventTick
  (params (DeltaSeconds :type Float%20%28single-precision%29))
  (CallFunction|UpdateStaticCamera DeltaSeconds))

(fn ConstructionScript)