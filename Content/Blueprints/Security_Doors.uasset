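; Two-panel sliding security door that opens for Mixamo_Jill when the ZombieMode HUD reports the key card, or unconditionally under other game modes.
; A trigger volume plays a timeline that lerps both panels between start and end positions, and any end overlap reverses it.
; The Construction Script creates dynamic materials on both panels, driving gloss and metal parameters from the first found KeyCard's spotlight color.
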(event OnComponentBeginOverlap(TriggerVolume)
  (params (OtherActor :type Actor%20Object%20Reference) (OtherComp :type Primitive%20Component%20Object%20Reference) (OtherBodyIndex :type Integer) (bFromSweep :type Boolean) (SweepResult :type Hit%20Result%20Structure%20%28by%20ref%29))
  (Utilities|Casting|CastToMixamo_Jill OtherActor)
  (bind _aszombie_mode (Utilities|Casting|CastToZombieMode (Game|GetGameMode))
    (:then
      (bind _yes (Default|HasItem (Variables|/Game/Modes/ZombieMode.ZombieMode_C|GetHUD_Widget _aszombie_mode) (Variables|Default|GetKeyCard)))
      (if _yes
        (bind _newtrack_1 (Timeline|Timeline_0 Play)
          (:Update
            (Utilities|FlowControl|Sequence
              (:then_0
                (Transformation|SetRelativeLocation (Variables|Default|GetDoor) (Math|Vector|Lerp(Vector) (Variables|Door|GetDoorStart) (Variables|Door|GetDoorEnd) _newtrack_1) false false))
              (:then_1
                (Transformation|SetRelativeLocation (Variables|Default|GetReverse) (Math|Vector|Lerp(Vector) (Variables|Door|GetReverseStart) (Variables|Door|GetReverseEnd) _newtrack_1) false false)))))))
    (:CastFailed
      (Timeline|Timeline_0 Play))))

(event OnComponentEndOverlap(TriggerVolume)
  (params (OtherActor :type Actor%20Object%20Reference) (OtherComp :type Primitive%20Component%20Object%20Reference) (OtherBodyIndex :type Integer))
  (bind _newtrack_1 (Timeline|Timeline_0 Reverse)
    (:Update
      (Utilities|FlowControl|Sequence
        (:then_0
          (Transformation|SetRelativeLocation (Variables|Default|GetDoor) (Math|Vector|Lerp(Vector) (Variables|Door|GetDoorStart) (Variables|Door|GetDoorEnd) _newtrack_1) false false))
        (:then_1
          (Transformation|SetRelativeLocation (Variables|Default|GetReverse) (Math|Vector|Lerp(Vector) (Variables|Door|GetReverseStart) (Variables|Door|GetReverseEnd) _newtrack_1) false false))))))

(fn ConstructionScript
  (bind _outactors (Actor|GetAllActorsOfClass (Variables|Default|GetKeyCard)))
  (for _array_element (Utilities|Array|MakeArray (Variables|Default|GetDoor) (Variables|Default|GetReverse))
    (bind _returnvalue (Rendering|Material|CreateDynamicMaterialInstance _array_element 0 0 :!class /Script/Engine.PrimitiveComponent))
    (bind _output_get (LocalVariables|SetDMI _returnvalue))
    (Rendering|Material|SetScalarParameterValue _output_get "R Gloss Int" (.r (Rendering|Components|Light|GetLightColor (Variables|/Game/Blueprints/BP_PickupKeyBase.BP_PickupKeyBase_C|GetSpotLight (Utilities|Array|Get(acopy) _outactors)))) :!class /Script/Engine.MaterialInstanceDynamic)
    (Rendering|Material|SetScalarParameterValue (LocalVariables|GetDMI) "R Metal Int" (.r (Rendering|Components|Light|GetLightColor (Variables|/Game/Blueprints/BP_PickupKeyBase.BP_PickupKeyBase_C|GetSpotLight (Utilities|Array|Get(acopy) _outactors)))) :!class /Script/Engine.MaterialInstanceDynamic)
    (Rendering|Material|SetScalarParameterValue _output_get "G Gloss Int" (.g (Rendering|Components|Light|GetLightColor (Variables|/Game/Blueprints/BP_PickupKeyBase.BP_PickupKeyBase_C|GetSpotLight (Utilities|Array|Get(acopy) _outactors)))) :!class /Script/Engine.MaterialInstanceDynamic)
    (Rendering|Material|SetScalarParameterValue (LocalVariables|GetDMI) "G Metal Int" (.g (Rendering|Components|Light|GetLightColor (Variables|/Game/Blueprints/BP_PickupKeyBase.BP_PickupKeyBase_C|GetSpotLight (Utilities|Array|Get(acopy) _outactors)))) :!class /Script/Engine.MaterialInstanceDynamic)
    (Rendering|Material|SetScalarParameterValue _output_get "B Gloss Int" (.b (Rendering|Components|Light|GetLightColor (Variables|/Game/Blueprints/BP_PickupKeyBase.BP_PickupKeyBase_C|GetSpotLight (Utilities|Array|Get(acopy) _outactors)))) :!class /Script/Engine.MaterialInstanceDynamic)
    (Rendering|Material|SetScalarParameterValue (LocalVariables|GetDMI) "B Metal Int" (.b (Rendering|Components|Light|GetLightColor (Variables|/Game/Blueprints/BP_PickupKeyBase.BP_PickupKeyBase_C|GetSpotLight (Utilities|Array|Get(acopy) _outactors)))) :!class /Script/Engine.MaterialInstanceDynamic)))