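; BP_PickupBase is a base pickup actor that the Mixamo_Jill character collects by overlapping its static mesh.
; On overlap it passes itself to AddItem on the ZombieMode game mode's HUD widget.
; A true result shows an "Inventory Full" toast; otherwise the pickup is hidden with collision disabled rather than destroyed.
; GetIcon exposes the pickup's Icon.
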(event OnComponentBeginOverlap(StaticMesh)
  (params (OtherActor :type Actor%20Object%20Reference) (OtherComp :type Primitive%20Component%20Object%20Reference) (OtherBodyIndex :type Integer) (bFromSweep :type Boolean) (SweepResult :type Hit%20Result%20Structure%20%28by%20ref%29))
  (Utilities|Casting|CastToMixamo_Jill OtherActor)
  (bind _aszombie_mode (Utilities|Casting|CastToZombieMode (Game|GetGameMode)))
  (bind _full (Default|AddItem (Variables|/Game/Modes/ZombieMode.ZombieMode_C|GetHUD_Widget _aszombie_mode) self))
  (if _full
    (Default|ShowToast (Variables|/Game/Modes/ZombieMode.ZombieMode_C|GetHUD_Widget _aszombie_mode) "Inventory Full")
    (else
      (Rendering|SetVisibility (Variables|Default|GetScene) false true)
      (Collision|SetActorEnableCollision false))))

(event EventBeginPlay)

(event EventActorBeginOverlap
  (params (OtherActor :type Actor%20Object%20Reference)))

(event EventTick
  (params (DeltaSeconds :type Float%20%28single-precision%29)))

(fn ConstructionScript)

(fn GetIcon
  (return (Variables|Pickup|GetIcon)))